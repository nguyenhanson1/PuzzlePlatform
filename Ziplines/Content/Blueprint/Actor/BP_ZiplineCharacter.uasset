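; BP_ZiplineCharacter is a character Blueprint that lets the player interact with nearby actors, named for use with ziplines.
; An InteractionCapsule overlap stores any actor implementing BP_InteractInterface as the single InteractActor, clearing it when that actor leaves.
; Pressing E sends InteractMessage to the stored actor, leaving the response to that actor.
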(event `self.InteractionCapsule.OnComponentBeginOverlap`
  (params (OverlappedComponent :type "PrimitiveComponent Object Reference") (OtherActor :type "Actor Object Reference") (OtherComp :type "PrimitiveComponent Object Reference") (OtherBodyIndex :type Integer) (bFromSweep :type Boolean) (SweepResult :type "HitResult Structure (by ref)"))
  (if (`KismetSystemLibrary.DoesImplementInterface` OtherActor "/Game/Blueprint/Interface/BP_InteractInterface.BP_InteractInterface_C")
    (set `self.InteractActor` OtherActor)))

(event `self.InteractionCapsule.OnComponentEndOverlap`
  (params (OverlappedComponent :type "PrimitiveComponent Object Reference") (OtherActor :type "Actor Object Reference") (OtherComp :type "PrimitiveComponent Object Reference") (OtherBodyIndex :type Integer))
  (if (== OtherActor (`self.InteractActor`))
    (set `self.InteractActor` null)))

(event `Key|E`
  (params (Key :type "Key Structure"))
  (:`Pressed`
    (message `/Game/Blueprint/Interface/BP_InteractInterface.Interact` (`self.InteractActor`))))

(fn `UserConstructionScript`
  (`parent.UserConstructionScript`))