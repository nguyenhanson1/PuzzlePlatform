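; Interactable zipline actor that carries the player along a spline, in either direction.
; The construction script fits a cable between the first two spline points and aligns a capsule along its length.
; Interact stops an active ride, or seeks a timeline to the player's distance ratio and plays or reverses it by facing dot product.
; Timeline updates place the player just below the spline, with play rate derived from Time.
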(event `self.ReceiveBeginPlay`
  (`TimelineComponent.SetPlayRate` (`self.Zipline Travel`) (/ 1.0 (`self.time`))))

(event `/Game/Blueprint/Interface/BP_InteractInterface.Interact`
  (bind _spline (`self.Spline`))
  (if (`TimelineComponent.IsPlaying` (`self.Zipline Travel`))
    (bind (_direction _traveldistance) (`Timeline|Zipline Travel` :!via `Stop` :!label _label)
      (:`Update`
        (bind (_returnvalue_x _returnvalue_y _returnvalue_z) (`KismetMathLibrary.BreakVector` (`SplineComponent.GetLocationAtDistanceAlongSpline` _spline (* _traveldistance (`SplineComponent.GetSplineLength` _spline)) "World")))
        (`self.K2_SetActorLocation` (`GameplayStatics.GetPlayerCharacter` 0) (`KismetMathLibrary.MakeVector` _returnvalue_x _returnvalue_y (- _returnvalue_z 100.0)) false false)))
    (else
      (`self.GetDistanceRatio`)
      (bind _returnvalue (`self.DetectDirection`))
      (if (>= _returnvalue 0.0)
        (goto _label)
        (else
          (goto _label :!via `Reverse`))))))

(fn `ConstructCable`
  (bind _cable (`self.Cable`))
  (`SceneComponent.K2_SetWorldLocation` (`self.Cable`) (`SplineComponent.GetLocationAtSplinePoint` (`self.Spline`) 0 "World") false false)
  (set `CableComponent.bAttachEnd` true _cable)
  (set `CableComponent.EndLocation` (`SplineComponent.GetLocationAtSplinePoint` (`self.Spline`) 1 "Local") _cable)
  (set `CableComponent.CableLength` (`SplineComponent.GetSplineLength` (`self.Spline`)) (`self.Cable`)))

(fn `ConstructCollision`
  (locals (LocalHalfLength :type "Float (double-precision)"))
  (bind _returnvalue (`SplineComponent.GetTransformAtDistanceAlongSpline` (`self.Spline`) (`local.LocalHalfLength`) "World" false))
  (bind _output_get (set `local.LocalHalfLength` (/ (`SplineComponent.GetSplineLength` (`self.Spline`)) 2.0)))
  (`CapsuleComponent.SetCapsuleHalfHeight` (`self.Capsule`) _output_get true)
  (`SceneComponent.K2_SetWorldTransform` (`self.Capsule`) (`KismetMathLibrary.MakeTransform` (.location _returnvalue) (`KismetMathLibrary.MakeRotator` (.roll (.rotation _returnvalue)) (+ (.pitch (.rotation _returnvalue)) 90.0) (.yaw (.rotation _returnvalue)))) false false))

(fn `DetectDirection`
  (returns (ReturnValue :type "Float (double-precision)"))
  (return (`KismetMathLibrary.Dot_VectorVector` (`KismetMathLibrary.GetForwardVector` (`SceneComponent.K2_GetComponentRotation` (`Character.Mesh` (`GameplayStatics.GetPlayerCharacter` 0)))) (`KismetMathLibrary.GetForwardVector` (`SceneComponent.K2_GetComponentRotation` (`self.Arrowfront`))))))

(fn `GetDistanceRatio`
  (bind _zipline_travel (`self.Zipline Travel`))
  (`TimelineComponent.SetNewTime` _zipline_travel (* (`TimelineComponent.GetTimelineLength` _zipline_travel) (/ (`KismetMathLibrary.VSize` (- (`self.K2_GetActorLocation` (`GameplayStatics.GetPlayerCharacter` 0)) (`SplineComponent.GetLocationAtSplinePoint` (`self.Spline`) 0 "World"))) (`SplineComponent.GetSplineLength` (`self.Spline`))))))

(fn `UserConstructionScript`
  (`self.ConstructCable`)
  (`self.ConstructCollision`))